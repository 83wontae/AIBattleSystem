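; BP_AICharacter is an AI character that starts with a test weapon, a skill set and an on-screen tag widget showing stamina.
; BeginPlay creates the tag in the viewport, attaches a collision-disabled BP_Weapon to the mesh's weapon socket, and initializes skills and tag values.
; The CharState component loads its base state from the DT_StateTable "Base" row on activation and pushes stamina changes to the tag through an event.
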(event OnComponentActivated(CharState)
  (params (Component :type Actor%20Component%20Object%20Reference) (bReset :type Boolean))
  (bind _returnvalue (Utilities|GetDataTableRow "/Game/AI/Data/DT_StateTable.DT_StateTable" "Base")
    (:then
      (Class|CharStateComponent|SetBaseState (Variables|Default|GetCharState) _returnvalue))))

(event EventUpdateSta(CharState)
  (params (CurSta :type Float%20%28single-precision%29) (MaxSta :type Float%20%28single-precision%29))
  (bind _chartag (Variables|Default|GetCharTag)
    (:then
      (Default|UpdateData _chartag CurSta MaxSta))
    (:else)))

(event EventBeginPlay
  (|CallParentFunction)
  (CallFunction|CreateTagWidget)
  (CallFunction|DoEquipTestWeapon)
  (CallFunction|InitData))

(fn ConstructionScript)

(fn CreateTagWidget
  (bind _returnvalue (UserInterface|CreateWidget "/Game/AI/Widget/CharTagWidget.CharTagWidget_C" 0 self))
  (bind _output_get (Variables|Default|SetCharTag _returnvalue))
  (UserInterface|Viewport|AddtoViewport _output_get 0))

(fn DoEquipTestWeapon
  (bind _returnvalue (Game|SpawnActorfromClass "/Game/AI/Blueprints/BP_Weapon.BP_Weapon_C" (Math|Transform|MakeTransform "0, 0, 0") "Undefined" "MultiplyWithRoot" 0 0))
  (bind _output_get (Variables|Default|SetEquipWeapon _returnvalue))
  (Collision|SetCollisionEnabled (Variables|/Game/AI/Blueprints/BP_Weapon.BP_Weapon_C|GetWeaponMesh _output_get) "NoCollision")
  (Transformation|AttachComponentToComponent _output_get (Variables|Character|GetMesh) "weapon" "SnapToTarget" "SnapToTarget" "KeepWorld" true))

(fn InitData
  (bind _charstate (Variables|Default|GetCharState))
  (Class|SkillComponent|SetSkillAT (Variables|Default|GetSkill) (Variables|Default|GetSkills))
  (bind _chartag (Variables|Default|GetCharTag)
    (:then
      (Default|UpdateData _chartag (Class|CharStateComponent|GetCurSta _charstate) (Class|CharStateComponent|GetMaxSta _charstate)))
    (:else)))